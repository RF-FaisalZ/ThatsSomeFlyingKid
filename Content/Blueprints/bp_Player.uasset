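; Player ship pawn that flies in the Y-Z plane, fires weapons, damages enemies it rams, and explodes at zero health, flagging death in bp_GameMode.
; A timeline flies it in before enabling Tick-driven movement with interpolated speeds and pitch tilt.
; Input-toggled gates and cooldown timers drive primary fire with random spread, or a fanned volley when powered up.
; Optional homing rockets alternate sides, targeting the last enemy overlapping the Locking component.
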(event OnComponentBeginOverlap(Locking)
  (params (OverlappedComponent :type Primitive%20Component%20Object%20Reference) (OtherActor :type Actor%20Object%20Reference) (OtherComp :type Primitive%20Component%20Object%20Reference) (OtherBodyIndex :type Integer) (bFromSweep :type Boolean) (SweepResult :type Hit%20Result%20Structure%20%28by%20ref%29))
  ;[1 1 1] Missile Locking
  (bind _asbp_enemy_base (Utilities|Casting|CastTobp_EnemyBase OtherActor))
  (bind _output_get (Variables|Default|SetEnemyLocked _asbp_enemy_base))
  (Game|SpawnActorfromClass "/Game/Blueprints/bpEnemyLockOn.bpEnemyLockOn_C" (Transformation|GetWorldTransform (Variables|Default|GetLocking)) "Undefined" 0 _output_get 0))

(event Custom|FireRateControl
  (bind _projectilespawn1 (Variables|Default|GetProjectileSpawn1))
  (bind _projectilespawn2 (Variables|Default|GetProjectileSpawn2))
  ;[1 0.6522 0.6123] Fire Control
  (Utilities|FlowControl|Sequence
    (:then_0
      (Variables|Floats|SetPrimaryFireRate (- (Variables|Floats|GetPrimaryFireRate) (Variables|Floats|GetDeltaSeconds)))
      (if (<= (Variables|Floats|GetPrimaryFireRate) 0.0)
        (Utilities|FlowControl|Gate true
          (:Exit
            (Variables|Floats|SetPrimaryFireRate (Variables|Floats|GetPrimaryFireRateBase))
            (if (Variables|Booleans|GetbHasPower)
              (CallFunction|PowerUpFire (Variables|Default|GetNumberOfPowerUpShots) _projectilespawn1 _projectilespawn2)
              (else
                (CallFunction|PrimaryFire _projectilespawn1 _projectilespawn2)))))))
    (:then_1
      (Variables|Floats|SetSecondaryFireRate (- (Variables|Floats|GetSecondaryFireRate) (Variables|Floats|GetDeltaSeconds)))
      (if (<= (Variables|Floats|GetSecondaryFireRate) 0.0)
        (Utilities|FlowControl|Gate true
          (:Exit
            (Variables|Floats|SetSecondaryFireRate (Variables|Floats|GetSecondaryFireRateBase))
            (if (Variables|Booleans|GetbHasSecondaryWeapon)
              (CallFunction|SecondaryFire (Variables|Default|GetSecondaryFire1) (Variables|Default|GetSecondaryFire2) (Variables|Default|GetEnemyLocked)))))))))

(event EventBeginPlay
  ;[0.6356 0.6414 1] Spawn Animation
  (Variables|Floats|SetCurrentHealth (Variables|Floats|GetMaxHealth))
  (Variables|Floats|SetPitch (.Pitch (Math|Rotator|BreakRotator (Variables|/Script/Engine.SceneComponent|GetRelativeRotation (Variables|Default|GetPlayerMesh)))))
  (Variables|Default|SetSpawnRotation (Transformation|GetWorldRotation (Variables|Default|GetPlayerMesh)))
  (Variables|Default|SetSpawnLocation (Transformation|GetActorLocation))
  (bind _spawn (Timeline|SpawnAnimation Play)
    (:Update
      (Transformation|SetActorLocation (Math|Vector|Lerp(Vector) (Variables|Default|GetSpawnLocation) (+ (Variables|Default|GetSpawnLocation) "0,1000.000000, 0") _spawn) false false)
      (Transformation|SetRelativeRotation (Variables|Default|GetPlayerMesh) (Math|Rotator|Lerp(Rotator) (Variables|Default|GetSpawnRotation) (Math|Rotator|MakeRotator 0.0 (+ (Variables|Floats|GetAnimationPitch) (Variables|Floats|GetPitch)) 0.0) _spawn) false false))
    (:Finished
      (Variables|Booleans|SetbMovementEnabled true))))

(event EventTick
  (params (DeltaSeconds :type Float%20%28single-precision%29))
  ;[0.7119 1 0.805] Movement
  (Variables|Floats|SetDeltaSeconds DeltaSeconds)
  (if (Variables|Booleans|GetbMovementEnabled)
    (CallFunction|FireRateControl)
    (Utilities|FlowControl|Sequence
      (:then_0
        (bind _returndirection (CallFunction|GetDirection (Variables|Floats|GetVerticalSpeed) (Input|AxisValues|GetMoveUp)))
        (Variables|Floats|SetVerticalSpeed _returndirection))
      (:then_1
        (bind _returndirection_2 (CallFunction|GetDirection (Variables|Floats|GetHorizontalSpeed) (Input|AxisValues|GetMoveRight)))
        (Variables|Floats|SetHorizontalSpeed _returndirection_2))
      (:then_2
        (Transformation|SetActorLocation (+ (Transformation|GetActorLocation) (Math|Vector|MakeVector 0.0 0.0 (Variables|Floats|GetVerticalSpeed))) true false)
        (Transformation|SetActorLocation (+ (Transformation|GetActorLocation) (Math|Vector|MakeVector 0.0 (Variables|Floats|GetHorizontalSpeed) 0.0)) true false)
        (if (> (Variables|Floats|GetCurrentHealth) 0.0)
          (Transformation|SetRelativeRotation (Variables|Default|GetPlayerMesh) (Math|Interpolation|RInterpTo (Transformation|GetActorRotation) (Math|Rotator|MakeRotator 0.0 (Variables|Floats|GetVerticalSpeed) 0.0) (Variables|Floats|GetDeltaSeconds) 8e+01) true false))))))

(event Game|Damage|EventAnyDamage
  (params (Damage :type Float%20%28single-precision%29) (DamageType :type Damage%20Type%20Object%20Reference) (InstigatedBy :type Controller%20Object%20Reference) (DamageCauser :type Actor%20Object%20Reference))
  ;[1 0.9846 0.5694] Player Death
  (Variables|Floats|SetCurrentHealth (Math|Float|Clamp(Float) (- (Variables|Floats|GetCurrentHealth) Damage) 0.0 (Variables|Floats|GetMaxHealth)))
  (if (<= (Variables|Floats|GetCurrentHealth) 0.0)
    (bind _asbp_game_mode (Utilities|Casting|CastTobp_GameMode (Game|GetGameMode)))
    (Variables|/Game/Blueprints/bp_GameMode.bp_GameMode_C|SetbPlayerDead _asbp_game_mode true)
    (Effects|SpawnEmitteratLocation "/Game/Particles/P_Explosion_Bomb.P_Explosion_Bomb" (Transformation|GetWorldLocation (Variables|Default|GetPlayerMesh)) "0, 0, 0" "8.000000,8.000000,8.000000")
    (Actor|DestroyActor)))

(event Collision|EventHit
  (params (MyComp :type Primitive%20Component%20Object%20Reference) (Other :type Actor%20Object%20Reference) (OtherComp :type Primitive%20Component%20Object%20Reference) (bSelfMoved :type Boolean) (HitLocation :type Vector :default "0, 0, 0") (HitNormal :type Vector :default "0, 0, 0") (NormalImpulse :type Vector :default "0, 0, 0") (Hit :type Hit%20Result%20Structure%20%28by%20ref%29))
  ;[1 1 1] Collision with Enemy Ships
  (bind _asbp_enemy_base (Utilities|Casting|CastTobp_EnemyBase Other))
  (Game|Damage|ApplyDamage _asbp_enemy_base 1e+02 0 0))

(event Input|ActionEvents|InputActionPrimaryFire
  (params (Key :type Key%20Structure))
  (bind _projectilespawn1 (Variables|Default|GetProjectileSpawn1))
  (bind _projectilespawn2 (Variables|Default|GetProjectileSpawn2))
  ;[1 0.6522 0.6123] Fire Control
  (:Pressed
    (Utilities|FlowControl|Gate true) ; enters at Open
  )
  (:Released
    (Utilities|FlowControl|Gate true) ; enters at Close
  ))

(event Input|ActionEvents|InputActionSecondaryFire
  (params (Key :type Key%20Structure))
  ;[1 0.6522 0.6123] Fire Control
  (:Pressed
    (Utilities|FlowControl|Gate true) ; enters at Open
  )
  (:Released
    (Utilities|FlowControl|Gate true) ; enters at Close
  ))

(fn ConstructionScript)

(fn GetDirection
  (params (Speed :type Float%20%28single-precision%29) (Direction :type Float%20%28single-precision%29))
  (bind _output_get (Variables|Floats|SetCurrentSpeed (Math|Interpolation|FInterpTo Speed (* (* Direction (Variables|Floats|GetMovementSpeed)) (Variables|Floats|GetDeltaSeconds)) (Variables|Floats|GetDeltaSeconds) 4.0)))
  (return _output_get))

(fn PrimaryFire
  (params (LeftFirePoint :type Scene%20Component%20Object%20Reference) (RightFirePoint :type Scene%20Component%20Object%20Reference))
  (Utilities|FlowControl|Sequence
    (:then_0
      (bind _returntransform (CallFunction|FireVariation (Transformation|GetWorldTransform LeftFirePoint)))
      (Game|SpawnActorfromClass "/Game/Blueprints/Projectiles/bp_ProjectilePlayerPrimary.bp_ProjectilePlayerPrimary_C" _returntransform "Undefined" 0 0)
      (Effects|SpawnEmitteratLocation "/Game/Particles/P_MuzzleFlash.P_MuzzleFlash" (Transformation|GetWorldLocation (Variables|Default|GetProjectileSpawn1)) "0, 0, 0" "10.000000,10.000000,10.000000"))
    (:then_1
      (bind _returntransform_2 (CallFunction|FireVariation (Transformation|GetWorldTransform RightFirePoint)))
      (Game|SpawnActorfromClass "/Game/Blueprints/Projectiles/bp_ProjectilePlayerPrimary.bp_ProjectilePlayerPrimary_C" _returntransform_2 "Undefined" 0 0)
      (Effects|SpawnEmitteratLocation "/Game/Particles/P_MuzzleFlash.P_MuzzleFlash" (Transformation|GetWorldLocation (Variables|Default|GetProjectileSpawn2)) "0, 0, 0" "10.000000,10.000000,10.000000"))))

(fn SecondaryFire
  (params (LeftFire :type Scene%20Component%20Object%20Reference%20%28by%20ref%29) (RightFire :type Scene%20Component%20Object%20Reference%20%28by%20ref%29) (LockedEnemy :type Bp%20Enemy%20Base%20Object%20Reference%20%28by%20ref%29))
  (if (Variables|Booleans|GetbCanFireSecondary)
    (Game|SpawnActorfromClass "/Game/Blueprints/Projectiles/bp_ProjectilePlayerRocketHoming.bp_ProjectilePlayerRocketHoming_C" (Transformation|GetWorldTransform LeftFire) "AlwaysSpawn" 0 (Variables|Default|GetEnemyLocked) 0)
    (else
      (Game|SpawnActorfromClass "/Game/Blueprints/Projectiles/bp_ProjectilePlayerRocketHoming.bp_ProjectilePlayerRocketHoming_C" (Transformation|GetWorldTransform RightFire) "AlwaysSpawn" 0 (Variables|Default|GetEnemyLocked) 0)))
  ;[1 1 1] Alternate The Firing Points
  (Variables|Booleans|SetbCanFireSecondary (not (Variables|Booleans|GetbCanFireSecondary)))
  (return))

(fn PowerUpFire
  (params (NumberOfShots :type Integer) (LeftFirePoint :type Scene%20Component%20Object%20Reference) (RightFirePoint :type Scene%20Component%20Object%20Reference))
  ;[1 1 1] PowerUp Fire Control
  (Utilities|FlowControl|Sequence
    (:then_0
      (bind _output_get (LocalVariables|SetOffsetLeft (/ NumberOfShots -2)))
      (LocalVariables|SetOffsetRight _output_get)
      (for _index (range 0 NumberOfShots)
        (Utilities|FlowControl|Sequence
          (:then_0
            (bind _returntransform (CallFunction|PowerUpFireVariation (Transformation|GetWorldTransform LeftFirePoint) (Math|Conversions|ToFloat(Integer) (LocalVariables|GetOffsetLeft))))
            (Game|SpawnActorfromClass "/Game/Blueprints/Projectiles/bp_ProjectilePlayerBase_Powered.bp_ProjectilePlayerBase_Powered_C" _returntransform "Undefined" 0 0)
            (LocalVariables|SetOffsetLeft (+ (LocalVariables|GetOffsetLeft) 1)))
          (:then_1
            (bind _returntransform_2 (CallFunction|PowerUpFireVariation (Transformation|GetWorldTransform RightFirePoint) (Math|Conversions|ToFloat(Integer) (LocalVariables|GetOffsetRight))))
            (Game|SpawnActorfromClass "/Game/Blueprints/Projectiles/bp_ProjectilePlayerBase_Powered.bp_ProjectilePlayerBase_Powered_C" _returntransform_2 "Undefined" 0 0)
            (LocalVariables|SetOffsetRight (+ (LocalVariables|GetOffsetRight) 1))))))
    (:then_1
      (Effects|SpawnEmitteratLocation "/Game/Particles/P_MuzzleFlash.P_MuzzleFlash" (Transformation|GetWorldLocation (Variables|Default|GetProjectileSpawn1)) "0, 0, 0" "15.000000,15.000000,15.000000"))
    (:then_2
      (Effects|SpawnEmitteratLocation "/Game/Particles/P_MuzzleFlash.P_MuzzleFlash" (Transformation|GetWorldLocation (Variables|Default|GetProjectileSpawn2)) "0, 0, 0" "15.000000,15.000000,15.000000"))))

(fn FireVariation
  (params (InputTransform :type Transform))
  (bind _location (Math|Transform|BreakTransform InputTransform))
  (return (Math|Transform|MakeTransform (Math|Vector|MakeVector (.x _location) (.y _location) (.z _location)) (Math|Rotator|MakeRotator (Math|Random|RandomFloatinRange -1.2 1.2) 0.0 0.0))))

(fn PowerUpFireVariation
  (params (InputTransform :type Transform) (Offset :type Float%20%28single-precision%29))
  (bind _location (Math|Transform|BreakTransform InputTransform))
  (return (Math|Transform|MakeTransform (Math|Vector|MakeVector (.x _location) (.y _location) (.z _location)) (Math|Rotator|MakeRotator (* Offset 5.0) 0.0 0.0))))

(fn FireRocket)