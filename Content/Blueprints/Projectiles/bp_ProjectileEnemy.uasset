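; Enemy projectile actor that flies forward and damages the player on contact.
; Each tick it moves along its local axes with a swept offset scaled by Speed and frame time.
; When the mesh begins overlapping a bp_Player, it spawns a hit particle and applies Damage; any overlap destroys it.
; The construction script sets the actor's size from its Scale variable.
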(event OnComponentBeginOverlap(ProjectileMesh)
  (params (OverlappedComponent :type Primitive%20Component%20Object%20Reference) (OtherActor :type Actor%20Object%20Reference) (OtherComp :type Primitive%20Component%20Object%20Reference) (OtherBodyIndex :type Integer) (bFromSweep :type Boolean) (SweepResult :type Hit%20Result%20Structure%20%28by%20ref%29))
  ;[1 1 1] Damage
  (bind _asbp_player (Utilities|Casting|CastTobp_Player OtherActor)
    (:then
      (Effects|SpawnEmitteratLocation "/Game/Particles/P_Hit.P_Hit" (Transformation|GetWorldLocation (Variables|Default|GetProjectileMesh)) "0, 0, 0" "20.000000,20.000000,20.000000")
      (Game|Damage|ApplyDamage _asbp_player (Variables|Default|GetDamage) 0 0))
    (:CastFailed
      _))
  (Actor|DestroyActor))

(event EventTick
  (params (DeltaSeconds :type Float%20%28single-precision%29))
  ;[1 1 1] Move Projectile
  (Variables|Default|SetDeltaSeconds DeltaSeconds)
  (Transformation|AddActorLocalOffset (* (Variables|Default|GetSpeed) (Variables|Default|GetDeltaSeconds)) true false))

(fn ConstructionScript
  (Transformation|SetActorScale3D (Variables|Default|GetScale)))