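; Base player rocket projectile that drops from its launch point, ignites and accelerates along world Y.
; A first timeline lerps the drop, then spawns ignition and smoke effects as a second timeline ramps velocity.
; HomingEnabled is set right after the drop, though no steering happens here, and Tick adds Speed-scaled velocity unless Hit.
; Any mesh overlap explodes and destroys the rocket, damaging only bp_EnemyBase actors.
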(event OnComponentBeginOverlap(ProjectileMesh)
  (params (OverlappedComponent :type Primitive%20Component%20Object%20Reference) (OtherActor :type Actor%20Object%20Reference) (OtherComp :type Primitive%20Component%20Object%20Reference) (OtherBodyIndex :type Integer) (bFromSweep :type Boolean) (SweepResult :type Hit%20Result%20Structure%20%28by%20ref%29))
  (bind _projectilemesh (Variables|Default|GetProjectileMesh))
  ;[1 1 1] Collision Events
  (bind _asbp_enemy_base (Utilities|Casting|CastTobp_EnemyBase OtherActor)
    (:then
      (Game|Damage|ApplyDamage _asbp_enemy_base (Variables|Default|GetDamage) 0 0))
    (:CastFailed
      _))
  (Rendering|SetVisibility _projectilemesh false false)
  (Effects|SpawnEmitteratLocation "/Game/Particles/P_Explosion_Fireball.P_Explosion_Fireball" (Transformation|GetWorldLocation _projectilemesh) "0, 0, 0" "12.000000,12.000000,12.000000")
  (Actor|DestroyActor))

(event EventBeginPlay
  (bind _particlesspawnlocation (Variables|Default|GetParticlesSpawnLocation))
  ;[1 1 1] Rocket Spawn and Speedup
  (Variables|Default|SetbHomingEnabled false)
  (bind _output_get (Variables|Default|SetSpawnLocation (Transformation|GetActorLocation)))
  (bind _track (Timeline|SpawnAnimation Play)
    (:Update
      (Transformation|SetActorLocation (Math|Vector|Lerp(Vector) _output_get (Math|Vector|MakeVector (.x (Variables|Default|GetSpawnLocation)) (+ (.y (Variables|Default|GetSpawnLocation)) (* _track 5e+01)) (- (.z (Variables|Default|GetSpawnLocation)) 1e+02)) _track) true false))
    (:Finished
      (Variables|Default|SetVectorSpeed (Math|Vector|Lerp(Vector) _output_get (Math|Vector|MakeVector (.x (Variables|Default|GetSpawnLocation)) (+ (.y (Variables|Default|GetSpawnLocation)) (* _track 5e+01)) (- (.z (Variables|Default|GetSpawnLocation)) 1e+02)) _track))
      (Effects|SpawnEmitteratLocation "/Game/Particles/P_Pixel_Explosion.P_Pixel_Explosion" (Transformation|GetWorldLocation _particlesspawnlocation) "0, 0, 0" "10.000000,10.000000,10.000000")
      (Effects|SpawnEmitterAttached "/Game/Particles/P_Smoke.P_Smoke" _particlesspawnlocation "None" "0, 0, 0" "0.000000,-180.000000, 0" "10.000000,10.000000,10.000000")
      (Utilities|FlowControl|Sequence
        (:then_0
          (bind _spawnanimation2 (Timeline|SpawnAnimation2 Play)
            (:Update
              (Variables|/Script/Engine.MovementComponent|SetVelocity (Variables|Default|GetProjectileMovement) (Math|Vector|Lerp(Vector) (Math|Vector|MakeVector 0.0 0.0 0.0) (Math|Vector|MakeVector 0.0 (* _spawnanimation2 2e+03) 0.0) _spawnanimation2)))
            (:Finished
              (Variables|Default|SetbHomingEnabled true :!label _label))))
        (:then_1
          (Rendering|ToggleVisibility (Variables|Default|GetPointLight) false)
          (goto _label))))))

(event EventTick
  (params (DeltaSeconds :type Float%20%28single-precision%29))
  ;[1 1 1] Missile Speedup
  (bind _output_get (Variables|Default|SetDeltaSeconds DeltaSeconds))
  (if (not (Variables|Default|GetbHit))
    (Variables|/Script/Engine.MovementComponent|SetVelocity (Variables|Default|GetProjectileMovement) (+ (Variables|/Script/Engine.MovementComponent|GetVelocity (Variables|Default|GetProjectileMovement)) (Math|Vector|MakeVector 0.0 (* _output_get (Variables|Default|GetSpeed)) 0.0)))))

(fn ConstructionScript)