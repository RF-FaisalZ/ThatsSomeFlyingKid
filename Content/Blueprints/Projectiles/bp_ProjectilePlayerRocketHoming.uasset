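; Player homing rocket projectile that steers toward its Enemy target while accelerating.
; Each Tick with a valid Enemy and homing enabled, it compounds RocketSpeedup by delta time and blends ProjectileMovement velocity toward the target direction at that speed, using a fixed, per-frame lerp alpha.
; With homing disabled and a valid Enemy, velocity is zeroed; without a valid Enemy, RocketSpeedup resets to its base value.
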(event EventBeginPlay
  (|CallParentFunction))

(event EventTick
  (params (DeltaSeconds :type Float%20%28single-precision%29))
  ;[1 1 1] Homimg Missile
  (|CallParentFunction DeltaSeconds)
  (Utilities|IsValid (Variables|Default|GetEnemy)
    (:Is%20Valid
      (if (Variables|Default|GetbHomingEnabled)
        (Variables|Default|SetRocketSpeedup (+ (* (Variables|Default|GetRocketSpeedup) (Variables|Default|GetDeltaSeconds)) (Variables|Default|GetRocketSpeedup)))
        (Variables|/Script/Engine.MovementComponent|SetVelocity (Variables|Default|GetProjectileMovement) (Math|Vector|Lerp(Vector) (Variables|/Script/Engine.MovementComponent|GetVelocity (Variables|Default|GetProjectileMovement)) (* (Math|Vector|Normalize (- (Transformation|GetActorLocation (Variables|Default|GetEnemy)) (Transformation|GetActorLocation))) (Variables|Default|GetRocketSpeedup)) 0.1))
        (else
          (Variables|/Script/Engine.MovementComponent|SetVelocity (Variables|Default|GetProjectileMovement) "0, 0, 0"))))
    (:Is%20Not%20Valid
      (Variables|Default|SetRocketSpeedup (Variables|Default|GetRocketSpeedBase)))))

(fn ConstructionScript
  (|CallParentFunction))