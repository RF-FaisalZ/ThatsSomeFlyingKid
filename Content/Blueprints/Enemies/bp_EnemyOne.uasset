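; EnemyOne is an enemy Blueprint that repeatedly fires projectiles at random intervals.
; After the parent Tick, a Delay between half a second and FireRate acts as the fire timer, since calls during a pending delay are ignored.
; Each completed delay spawns a small Bp_ProjectileEnemy at ProjectileSpawn, passing it Damage and a fixed velocity along negative Y.
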(event EventBeginPlay
  (|CallParentFunction))

(event EventTick
  (params (DeltaSeconds :type Float%20%28single-precision%29))
  (|CallParentFunction DeltaSeconds)
  (Utilities|FlowControl|Delay (Math|Random|RandomFloatinRange 0.5 (Variables|Default|GetFireRate)))
  (Game|SpawnActorfromClass "/Game/Blueprints/Projectiles/bp_ProjectileEnemy.bp_ProjectileEnemy_C" (Transformation|GetWorldTransform (Variables|Default|GetProjectileSpawn)) "Undefined" 0 (Variables|Default|GetDamage) "0.000000,-5000.000000,0.000000" "0.200000,0.200000,0.200000" 0))

(fn ConstructionScript
  (|CallParentFunction))