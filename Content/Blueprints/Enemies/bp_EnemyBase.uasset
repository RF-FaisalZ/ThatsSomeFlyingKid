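; Base enemy Blueprint that sweeps in on spawn, patrols back and forth and reports itself to bp_GameMode's live enemy count.
; A timeline lerps it a random distance along negative Y, then Tick moves it along Z with swept collision.
; Hits reroll speed and, until it has damaged the player once, reverse direction on non-enemy contact.
; Damage drains clamped health; at zero it decrements the count, explodes and destroys itself.
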(event Collision|EventHit
  (params (MyComp :type Primitive%20Component%20Object%20Reference) (Other :type Actor%20Object%20Reference) (OtherComp :type Primitive%20Component%20Object%20Reference) (bSelfMoved :type Boolean) (HitLocation :type Vector :default "0, 0, 0") (HitNormal :type Vector :default "0, 0, 0") (NormalImpulse :type Vector :default "0, 0, 0") (Hit :type Hit%20Result%20Structure%20%28by%20ref%29))
  ;[1 1 1] Death
  (Variables|Floats|SetMovementSpeed (Math|Random|RandomFloatinRange (Variables|Floats|GetMovementSpeedMin) (Variables|Floats|GetMovementSpeedMax)))
  (if (not (Variables|Default|GetbPlayerHit))
    (Utilities|Casting|CastTobp_EnemyBase Other
      (:CastFailed
        (Variables|Default|SetbMoveDirection (not (Variables|Default|GetbMoveDirection)))
        (bind _asbp_player (Utilities|Casting|CastTobp_Player Other))
        (Game|Damage|ApplyDamage _asbp_player 5e+01 0 0)
        (Variables|Default|SetbPlayerHit true)))))

(event Game|Damage|EventAnyDamage
  (params (Damage :type Float%20%28single-precision%29) (DamageType :type Damage%20Type%20Object%20Reference) (InstigatedBy :type Controller%20Object%20Reference) (DamageCauser :type Actor%20Object%20Reference))
  (bind _gamemode (Variables|Default|GetGameMode))
  ;[1 1 1] Death
  (Variables|Floats|SetHealth (Math|Float|Clamp(Float) (- (Variables|Floats|GetHealth) Damage) 0.0 (Variables|Floats|GetMaxHealth)))
  (if (<= (Variables|Floats|GetHealth) 0.0)
    (Variables|/Game/Blueprints/bp_GameMode.bp_GameMode_C|SetLiveEnemies _gamemode (- (Variables|/Game/Blueprints/bp_GameMode.bp_GameMode_C|GetLiveEnemies _gamemode) 1))
    (Utilities|FlowControl|Delay 0.1)
    (Effects|SpawnEmitteratLocation "/Game/Particles/P_Explosion_Bomb.P_Explosion_Bomb" (Transformation|GetActorLocation) "0, 0, 0" (Variables|Default|GetScale))
    (Variables|Default|SetbPlayerHit false)
    (Actor|DestroyActor)))

(event EventBeginPlay
  ;[1 1 1] Control Random Movement
  (bind _asbp_game_mode (Utilities|Casting|CastTobp_GameMode (Game|GetGameMode)))
  (bind _output_get (Variables|Default|SetGameMode _asbp_game_mode))
  (Variables|/Game/Blueprints/bp_GameMode.bp_GameMode_C|SetLiveEnemies _output_get (+ (Variables|/Game/Blueprints/bp_GameMode.bp_GameMode_C|GetLiveEnemies _output_get) 1))
  (Variables|Default|SetbMoveDirection (Math|Random|RandomBool))
  (Variables|Floats|SetMovementSpeed (Math|Random|RandomFloatinRange (Variables|Floats|GetMovementSpeedMin) (Variables|Floats|GetMovementSpeedMax)))
  (Variables|Floats|SetSweepIn (Math|Random|RandomFloatinRange 1e+03 1.7e+03))
  ;[1 1 1] Spawn Animation
  (Variables|Default|SetSpawnLocation (Transformation|GetActorLocation))
  (bind _newtrack_0 (Timeline|SpawnAnimation Play)
    (:Update
      (Transformation|SetActorLocation (Math|Vector|Lerp(Vector) (Variables|Default|GetSpawnLocation) (- (Variables|Default|GetSpawnLocation) (Math|Vector|MakeVector 0.0 (Variables|Floats|GetSweepIn) 0.0)) _newtrack_0) false false))
    (:Finished
      (Variables|Default|SetbMoveEnabled true))))

(event EventTick
  (params (DeltaSeconds :type Float%20%28single-precision%29))
  ;[1 1 1] Enemy Movement
  (Variables|Floats|SetDeltaSeconds DeltaSeconds)
  (if (Variables|Default|GetbMoveEnabled)
    (Transformation|SetActorLocation (+ (Transformation|GetActorLocation) (* (Math|Vector|RotateVector (Math|Vector|MakeVector 0.0 0.0 (* (Variables|Floats|GetMovementSpeed) (Math|Float|SelectFloat 1.0 -1.0 (Variables|Default|GetbMoveDirection)))) "0, 0, 0") (Variables|Floats|GetDeltaSeconds))) true false)))

(fn ConstructionScript
  (Variables|Floats|SetHealth (Variables|Floats|GetMaxHealth)))